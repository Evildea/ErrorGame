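; Music visualiser controller that builds two vertical columns of platforms, plays the music, shows the game UI and raises the water.
; BeginPlay finds the left and right markers and Water actor, then SpawnPlatforms stacks platforms at each marker.
; Each tick samples the music's frequency spectrum at game time, and MakeScale stretches each platform's Y by its band, both columns sharing bands.
; Water rises inside that per-platform loop.
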(event `self.ReceiveBeginPlay`
  ;[1 1 1] Get Spawn Locations
  (bind _outactors (`GameplayStatics.GetAllActorsOfClass` "/Game/GameObjects/Blueprints/PlatformLeftLocation.PlatformLeftLocation_C"))
  (set `self.LeftSpawn` (`|GetArrayItem` _outactors))
  (bind _outactors_2 (`GameplayStatics.GetAllActorsOfClass` "/Game/GameObjects/Blueprints/PlatformRightLocation.PlatformRightLocation_C"))
  (set `self.RightSpawn` (`|GetArrayItem` _outactors_2))
  (bind _outactors_3 (`GameplayStatics.GetAllActorsOfClass` "/Game/GameObjects/Blueprints/Water.Water_C"))
  (set `self.Water` (`|GetArrayItem` _outactors_3))
  (`self.SpawnPlatforms` (`self.NumberOfPlatforms`) (`self.K2_GetActorLocation` (`self.LeftSpawn`)))
  (`self.SpawnPlatforms` (`self.NumberOfPlatforms`) (`self.K2_GetActorLocation` (`self.RightSpawn`)))
  (`GameplayStatics.PlaySound2D` (`self.Music`) 1.0 1.0 0.0 null null)
  (bind _returnvalue (`|CreateWidget` "/Game/UI/GameUI.GameUI_C"))
  (`UserWidget.AddToViewport` _returnvalue 0))

(event `self.ReceiveTick`
  (params (DeltaSeconds :type "Float (single-precision)"))
  (`GameplayStatics.PlaySound2D` null 1.0 1.0 0.0 null null)
  (bind _outspectrum (`SoundVisualizationStatics.CalculateFrequencySpectrum` (`self.Music`) 0 (`KismetSystemLibrary.GetGameTimeInSeconds`) 0.1 (`self.NumberOfPlatforms`)))
  (set `self.Spectrum` _outspectrum)
  (for (_array_element _array_index) (`self.ListOfPlatforms`)
    (if (>= _array_index (`self.NumberOfPlatforms`))
      (bind _output (`self.MakeScale` (- (- _array_index (`self.NumberOfPlatforms`)) 1)))
      (`self.SetActorScale3D` _array_element _output)
      (else
        (bind _output_2 (`self.MakeScale` _array_index))
        (`self.SetActorScale3D` _array_element _output_2)))
    (`self.K2_SetActorLocation` (`self.Water`) (`KismetMathLibrary.MakeVector` (.x (`self.K2_GetActorLocation` (`self.Water`))) (.y (`self.K2_GetActorLocation` (`self.Water`))) (+ (.z (`self.K2_GetActorLocation` (`self.Water`))) (* (`GameplayStatics.GetWorldDeltaSeconds`) (`self.WaterSpeed`)))) false false)))

(fn `MakeScale`
  (params (Index :type Integer))
  (returns (Output :type "Vector Structure"))
  (return (`KismetMathLibrary.MakeVector` 1.0 (`KismetMathLibrary.FMax` (`KismetMathLibrary.MultiplyMultiply_FloatFloat` (* (`KismetMathLibrary.Abs` (`|GetArrayItem` (`self.Spectrum`) Index)) 0.05) (`self.Power`)) 1.0) 1.0)))

(fn `SpawnPlatforms`
  (params (NumberOfPlatforms :type Integer) (SpawnLocationStart :type "Vector Structure"))
  (locals (SpawnHeight :type Integer))
  (for _index (range (+ NumberOfPlatforms 1))
    (`/Engine/EditorBlueprintResources/StandardMacros.IncrementInt` (`local.SpawnHeight`)
      (:`  `
        (bind _returnvalue (`|SpawnActorFromClass` "/Game/GameObjects/Blueprints/Platform.Platform_C" (`KismetMathLibrary.MakeTransform` (`KismetMathLibrary.MakeVector` (.x SpawnLocationStart) (.y SpawnLocationStart) (* _index (`self.SeperationDistance`)))) "Undefined" "OverrideRootScale" null null))
        (`KismetArrayLibrary.Array_Add` (`self.ListOfPlatforms`) _returnvalue)))))

(fn `UserConstructionScript`)