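; PlatformController builds a row of music-reactive platforms, creates the game UI and starts the music after a delay.
; BeginPlay spawns dummy and repeated spectrum platforms along Y from the first PlatformSpawnLocation.
; While music plays, Tick samples its frequency spectrum at the elapsed playback time.
; MakeScale wraps platform indices around the spectrum, turning magnitudes into power-curved, clamped X scales for platforms beyond the dummy range.
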(event `self.ReceiveBeginPlay`
  ;[1 1 1] Get Spawn Locations
  (bind _outactors (`GameplayStatics.GetAllActorsOfClass` "/Game/GameObjects/Blueprints/PlatformSpawnLocation.PlatformSpawnLocation_C"))
  (set `self.SpawnLocation` (`|GetArrayItem` _outactors))
  (`self.SpawnPlatforms` (* (`self.RepeatMusic`) (`self.NumberOfPlatforms`)) (`self.K2_GetActorLocation` (`self.SpawnLocation`)))
  (bind _returnvalue (`|CreateWidget` "/Game/UI/GameUI.GameUI_C"))
  (`UserWidget.AddToViewport` _returnvalue 0)
  (`KismetSystemLibrary.Delay` (`self.DelayMusicStart`))
  (`GameplayStatics.PlaySound2D` (`self.Music`) 1.0 1.0 0.0 null null)
  (set `self.PlayMusic` true))

(event `self.ReceiveTick`
  (params (DeltaSeconds :type "Float (single-precision)"))
  (if (`self.PlayMusic`)
    (`GameplayStatics.PlaySound2D` null 1.0 1.0 0.0 null null)
    (bind _outspectrum (`SoundVisualizationStatics.CalculateFrequencySpectrum` (`self.Music`) 0 (- (`KismetSystemLibrary.GetGameTimeInSeconds`) (`self.DelayMusicStart`)) 0.1 (`self.NumberOfPlatforms`)))
    (set `self.Spectrum` _outspectrum)
    (for (_array_element _array_index) (`self.ListOfPlatforms`)
      (if (> _array_index (`self.NumberOfDummyPlatforms`))
        (bind _output (`self.MakeScale` _array_index))
        (`self.SetActorScale3D` _array_element _output)
        (else
          (`self.SetActorScale3D` (1.0 1.0 1.0)))))
    (else
      (for _array_element_2 (`self.ListOfPlatforms`)
        (`self.SetActorScale3D` _array_element_2 (1.0 1.0 1.0))))))

(fn `MakeScale`
  (params (Index :type Integer))
  (returns (Output :type "Vector Structure"))
  (locals (IndexLocal :type Integer))
  (set `local.IndexLocal` Index)
  (while (> (`local.IndexLocal`) (`KismetArrayLibrary.Array_Length` (`self.Spectrum`)))
    (if (> (`local.IndexLocal`) (`KismetArrayLibrary.Array_Length` (`self.Spectrum`)))
      (set `local.IndexLocal` (- (`local.IndexLocal`) (`KismetArrayLibrary.Array_Length` (`self.Spectrum`))))))
  (return (`KismetMathLibrary.MakeVector` (`KismetMathLibrary.FMin` (`self.HeightCap`) (`KismetMathLibrary.FMax` (`KismetMathLibrary.MultiplyMultiply_FloatFloat` (* (`KismetMathLibrary.Abs` (`|GetArrayItem` (`self.Spectrum`) (`local.IndexLocal`))) 0.05) (`self.Power`)) 1.0)) 1.0 1.0)))

(fn `SpawnPlatforms`
  (params (NumberOfPlatforms :type Integer) (SpawnLocationStart :type "Vector Structure"))
  (locals (SpawnHeight :type Integer))
  (for _index (range (+ (+ (`self.NumberOfDummyPlatforms`) NumberOfPlatforms) 1))
    (`/Engine/EditorBlueprintResources/StandardMacros.IncrementInt` (`local.SpawnHeight`)
      (:`  `
        (bind _returnvalue (`|SpawnActorFromClass` "/Game/GameObjects/Blueprints/Platform.Platform_C" (`KismetMathLibrary.MakeTransform` (`KismetMathLibrary.MakeVector` (.x SpawnLocationStart) (* _index (`self.SeperationDistance`)) (.z SpawnLocationStart))) "Undefined" "OverrideRootScale" null null))
        (`KismetArrayLibrary.Array_Add` (`self.ListOfPlatforms`) _returnvalue)))))

(fn `UserConstructionScript`)