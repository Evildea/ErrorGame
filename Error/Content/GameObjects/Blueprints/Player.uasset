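; Player Blueprint that moves itself along Y each tick, scores points over time and can briefly phase out to avoid platforms.
; PhaseOut input toggles a flag for a set duration and switches the Ghost material parameter collection.
; Tick disables sphere collision while phased and otherwise uses a Delay as the points timer.
; Overlapping a Platform while solid shows the GameOver widget and pauses the game.
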(event `InputAction|PhaseOut`
  (params (Key :type "Key Structure"))
  (:`Pressed`
    (if (not (`self.isPhasedOut`))
      (set `self.isPhasedOut` true)
      (`KismetMaterialLibrary.SetScalarParameterValue` "/Game/Character/Material/Ghost.Ghost" "Mat Switch")
      (`KismetSystemLibrary.Delay` (`self.PhaseOutDuration`))
      (`KismetMaterialLibrary.SetScalarParameterValue` "/Game/Character/Material/Ghost.Ghost" "Mat Switch" 1.0)
      (set `self.isPhasedOut` false))))

(event `self.ReceiveBeginPlay`)

(event `self.ReceiveTick`
  (params (DeltaSeconds :type "Float (single-precision)"))
  (bind (_returnvalue_x _returnvalue_y _returnvalue_z) (`KismetMathLibrary.BreakVector` (`self.K2_GetActorLocation`)))
  (bind _sphere (`self.Sphere`))
  (set `self.DeltaTime` DeltaSeconds)
  (`self.K2_SetActorLocation` (`KismetMathLibrary.MakeVector` _returnvalue_x (+ (* (`self.Speed`) (`self.DeltaTime`)) _returnvalue_y) _returnvalue_z))
  (if (`self.isPhasedOut`)
    (`PrimitiveComponent.SetCollisionEnabled` _sphere "NoCollision")
    (else
      (`PrimitiveComponent.SetCollisionEnabled` _sphere "QueryAndPhysics")
      ;[1 1 1] Timer
      (`KismetSystemLibrary.Delay` (`self.PointCountSpeed`))
      (if (not (`self.isPhasedOut`))
        (`/Engine/EditorBlueprintResources/StandardMacros.IncrementInt` (`self.Points`))))))

(event `self.ReceiveActorBeginOverlap`
  (params (OtherActor :type "Actor Object Reference"))
  (cast `/Game/GameObjects/Blueprints/Platform` OtherActor)
  (if (not (`self.isPhasedOut`))
    (bind _returnvalue (`|CreateWidget` "/Game/UI/GameOver.GameOver_C"))
    (bind _output_get (set `self.Restart` _returnvalue))
    (`UserWidget.AddToViewport` _output_get 0)
    (`WidgetBlueprintLibrary.SetInputMode_UIOnlyEx` (`GameplayStatics.GetPlayerController` 0) (`self.Restart`))
    (set `PlayerController.bShowMouseCursor` true (`GameplayStatics.GetPlayerController` 0))
    (`GameplayStatics.SetGamePaused` true)))

(fn `UserConstructionScript`)